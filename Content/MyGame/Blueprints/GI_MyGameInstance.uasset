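; Game instance that saves, loads and clears player and wave progress through a BP_SaveGame slot.
; SaveGameData creates CurrentSave if needed, copies in player health, coins, key, slow spell and first BP_WaveTrigger state, then writes the slot.
; LoadGameData only caches the slot in CurrentSave; ApplyLoadedDataToWorld separately pushes it onto player and trigger.
; ClearGameData deletes the slot but leaves CurrentSave in memory.
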(fn `ApplyLoadedDataToWorld`
  (`/Engine/EditorBlueprintResources/StandardMacros.IsValid` (`self.currentSave`)
    (:`Is Valid`
      (if true
        (bind _asbp_first_person_character (cast `/Game/MyGame/Blueprints/MyCharacter/BP_FirstPersonCharacter` (`GameplayStatics.GetPlayerCharacter` 0)))
        (set `/Game/MyGame/Blueprints/MyCharacter/BP_FirstPersonCharacter.currentHealth` (`/Game/MyGame/Blueprints/BP_SaveGame.savedPlayerHealth` (`self.currentSave`)) _asbp_first_person_character)
        (set `/Game/MyGame/Blueprints/MyCharacter/BP_FirstPersonCharacter.coinsCollected` (`/Game/MyGame/Blueprints/BP_SaveGame.savedCoinsCollected` (`self.currentSave`)) _asbp_first_person_character)
        (set `/Game/MyGame/Blueprints/MyCharacter/BP_FirstPersonCharacter.hasKey` (`/Game/MyGame/Blueprints/BP_SaveGame.SavedHasKey` (`self.currentSave`)) _asbp_first_person_character)
        (set `/Game/MyGame/Blueprints/MyCharacter/BP_FirstPersonCharacter.hasSlowSpell` (`/Game/MyGame/Blueprints/BP_SaveGame.savedHasSlowSpell` (`self.currentSave`)) _asbp_first_person_character)
        (bind _outactors (`GameplayStatics.GetAllActorsOfClass` "/Game/MyGame/Blueprints/BP_WaveTrigger.BP_WaveTrigger_C"))
        (bind _output (`|GetArrayItem` _outactors))
        (set `/Game/MyGame/Blueprints/BP_WaveTrigger.waveNumber` (`/Game/MyGame/Blueprints/BP_SaveGame.savedCurrentWave` (`self.currentSave`)) _output)
        (set `/Game/MyGame/Blueprints/BP_WaveTrigger.enemiesToSpawn` (`/Game/MyGame/Blueprints/BP_SaveGame.savedEnemiesToSpawn` (`self.currentSave`)) _output)
        (else
          (return))))))

(fn `ClearGameData`
  (`GameplayStatics.DeleteGameInSlot` (`self.saveSlotName`))
  (`KismetSystemLibrary.PrintString` "CLEARED GAME DATA"))

(fn `LoadGameData`
  (bind _returnvalue (`GameplayStatics.DoesSaveGameExist` (`self.saveSlotName`)))
  (if _returnvalue
    (bind _returnvalue_2 (`GameplayStatics.LoadGameFromSlot` (`self.saveSlotName`)))
    (bind _asbp_save_game (cast `/Game/MyGame/Blueprints/BP_SaveGame` _returnvalue_2))
    (set `self.currentSave` _asbp_save_game)))

(fn `SaveGameData`
  (`/Engine/EditorBlueprintResources/StandardMacros.IsValid` (`self.currentSave`)
    (:`Is Valid`
      (`KismetSystemLibrary.PrintString` "BRANCH TRUE FIRED"))
    (:`Is Not Valid`
      (`KismetSystemLibrary.PrintString` "BRANCH FALSE FIRED")
      (bind _returnvalue (`GameplayStatics.CreateSaveGameObject` "/Game/MyGame/Blueprints/BP_SaveGame.BP_SaveGame_C"))
      (`KismetSystemLibrary.PrintString` "SAVE: CREATED NEW SAVE OBJECT")
      (set `self.currentSave` _returnvalue)))
  (bind _asbp_first_person_character (cast `/Game/MyGame/Blueprints/MyCharacter/BP_FirstPersonCharacter` (`GameplayStatics.GetPlayerCharacter` 0)))
  (`KismetSystemLibrary.PrintString` (`KismetStringLibrary.Concat_StrStr` "player haskey =" (`KismetStringLibrary.Conv_BoolToString` (`/Game/MyGame/Blueprints/MyCharacter/BP_FirstPersonCharacter.hasKey` _asbp_first_person_character))))
  (bind _outactors (`GameplayStatics.GetAllActorsOfClass` "/Game/MyGame/Blueprints/BP_WaveTrigger.BP_WaveTrigger_C"))
  (set `/Game/MyGame/Blueprints/BP_SaveGame.savedPlayerHealth` (`/Game/MyGame/Blueprints/MyCharacter/BP_FirstPersonCharacter.currentHealth` _asbp_first_person_character) (`self.currentSave`))
  (set `/Game/MyGame/Blueprints/BP_SaveGame.savedCoinsCollected` (`/Game/MyGame/Blueprints/MyCharacter/BP_FirstPersonCharacter.coinsCollected` _asbp_first_person_character) (`self.currentSave`))
  (set `/Game/MyGame/Blueprints/BP_SaveGame.SavedHasKey` (`/Game/MyGame/Blueprints/MyCharacter/BP_FirstPersonCharacter.hasKey` _asbp_first_person_character) (`self.currentSave`))
  (bind _output (`|GetArrayItem` _outactors))
  (set `/Game/MyGame/Blueprints/BP_SaveGame.savedCurrentWave` (`/Game/MyGame/Blueprints/BP_WaveTrigger.waveNumber` _output) (`self.currentSave`))
  (set `/Game/MyGame/Blueprints/BP_SaveGame.savedEnemiesToSpawn` (`/Game/MyGame/Blueprints/BP_WaveTrigger.enemiesToSpawn` _output) (`self.currentSave`))
  (set `/Game/MyGame/Blueprints/BP_SaveGame.savedHasSlowSpell` (`/Game/MyGame/Blueprints/MyCharacter/BP_FirstPersonCharacter.hasSlowSpell` _asbp_first_person_character) (`self.currentSave`))
  (`GameplayStatics.SaveGameToSlot` (`self.currentSave`) (`self.saveSlotName`))
  (`KismetSystemLibrary.PrintString` "GAME SAVED'"))