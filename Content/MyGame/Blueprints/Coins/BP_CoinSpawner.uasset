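; BP_CoinSpawner is a coin spawner actor meant to scatter BP_Coin actors within its Box component.
; On BeginPlay, a DoN looped back on itself calls SpawnCoin until the count reaches AmountOfCoins.
; SpawnCoin's entry is unwired, so it currently spawns nothing.
; Its disconnected logic would trace down from a random point in the box and spawn a coin at the hit location.
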(event `self.ReceiveBeginPlay`
  (bind _counter (`/Engine/EditorBlueprintResources/StandardMacros.Do N` (`self.amountOfCoins`) :!label _label)
    (:`Exit`
      (`self.SpawnCoin`)
      (if (not (== _counter (`self.amountOfCoins`)))
        (goto _label)))))

(fn `SpawnCoin`)

(fn `UserConstructionScript`)