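; BP_ShopKeeper is a shopkeeper that signals when the player can interact with it.
; On BeginPlay it caches the player character as BP_FirstPersonCharacter.
; Overlap begin and end on InteractionTrigger show or hide InteractWidget and set CanInteract on that cached player, without checking which actor overlapped.
; The shop interaction itself is not handled here, and begin overlap also prints a debug string.
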(event `self.ReceiveBeginPlay`
  (bind _asbp_first_person_character (cast `/Game/MyGame/Blueprints/MyCharacter/BP_FirstPersonCharacter` (`GameplayStatics.GetPlayerCharacter` 0)))
  (set `self.playerRef` _asbp_first_person_character))

(event `self.Interaction Trigger.OnComponentBeginOverlap`
  (params (OverlappedComponent :type "PrimitiveComponent Object Reference") (OtherActor :type "Actor Object Reference") (OtherComp :type "PrimitiveComponent Object Reference") (OtherBodyIndex :type Integer) (bFromSweep :type Boolean) (SweepResult :type "HitResult Structure (by ref)"))
  ; Set visibility of interaction prompt
  (`KismetSystemLibrary.PrintString` "BEGIN OVERLAP FIRED")
  (`SceneComponent.SetVisibility` (`self.Interact Widget`) true false)
  (set `/Game/MyGame/Blueprints/MyCharacter/BP_FirstPersonCharacter.canInteract` true (`self.playerRef`)))

(event `self.Interaction Trigger.OnComponentEndOverlap`
  (params (OverlappedComponent :type "PrimitiveComponent Object Reference") (OtherActor :type "Actor Object Reference") (OtherComp :type "PrimitiveComponent Object Reference") (OtherBodyIndex :type Integer))
  ; Set visibility of interaction prompt
  (`SceneComponent.SetVisibility` (`self.Interact Widget`) false false)
  (set `/Game/MyGame/Blueprints/MyCharacter/BP_FirstPersonCharacter.canInteract` false (`self.playerRef`)))

(fn `UserConstructionScript`)