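; BP_Projectile_Knockback is a projectile that knocks back nearby BP_EnemyAI characters when its collision sphere hits something.
; On hit, it runs a sphere overlap for pawns at the impact point within KnockbackRadius, ignoring itself and its owner.
; Each enemy found is launched away from the projectile by KnockbackAmount with a slight upward lift, overriding its current velocity.
; The graph applies no damage and does not destroy the projectile.
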(event `self.CollisionSphere.OnComponentHit`
  (params (HitComponent :type "PrimitiveComponent Object Reference") (OtherActor :type "Actor Object Reference") (OtherComp :type "PrimitiveComponent Object Reference") (NormalImpulse :type "Vector Structure") (Hit :type "HitResult Structure (by ref)"))
  (bind _outactors (`KismetSystemLibrary.SphereOverlapActors` (`.ImpactPoint` (`GameplayStatics.BreakHitResult` Hit)) (`self.knockbackRadius`) (`|MakeArray` "ObjectTypeQuery3" :!type "EObjectTypeQuery Enum") null (`|MakeArray` self (`self.GetOwner`) :!type "Actor Object Reference")))
  (for _array_element _outactors
    (bind _asbp_enemy_ai (cast `/Game/MyGame/Blueprints/EnemyAI/BP_EnemyAI` _array_element))
    (bind (_returnvalue_x _returnvalue_y _returnvalue_z) (`KismetMathLibrary.BreakVector` (* (`KismetMathLibrary.Normal` (- (`self.K2_GetActorLocation` _asbp_enemy_ai) (`self.K2_GetActorLocation`))) (`self.knockbackAmount`))))
    (`Character.LaunchCharacter` _asbp_enemy_ai (`KismetMathLibrary.MakeVector` _returnvalue_x _returnvalue_y (+ _returnvalue_z 20.0)) true true)))

(fn `UserConstructionScript`
  (`parent.UserConstructionScript`))