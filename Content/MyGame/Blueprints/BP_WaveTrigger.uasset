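; Wave trigger actor that starts an escalating enemy wave when the first-person player enters its box while no wave is active.
; It spawns BP_EnemyAI at randomly picked spawn points with an X offset and raised Z, re-rolling the point for each transform component.
; Death events decrement the alive count and update the player's wave UI.
; At zero, the wave ends, increasing the wave number and next enemy count.
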(event `self.ReceiveBeginPlay`
  (bind _asbp_first_person_character (cast `/Game/MyGame/Blueprints/MyCharacter/BP_FirstPersonCharacter` (`GameplayStatics.GetPlayerCharacter` 0)))
  (set `self.playerRef` _asbp_first_person_character))

(event `self.Box.OnComponentBeginOverlap`
  (params (OverlappedComponent :type "PrimitiveComponent Object Reference") (OtherActor :type "Actor Object Reference") (OtherComp :type "PrimitiveComponent Object Reference") (OtherBodyIndex :type Integer) (bFromSweep :type Boolean) (SweepResult :type "HitResult Structure (by ref)"))
  (cast `/Game/MyGame/Blueprints/EnemyAI/BP_EnemyAI` OtherActor
    (:`CastFailed`
      (cast `/Game/MyGame/Blueprints/MyCharacter/BP_FirstPersonCharacter` OtherActor)
      (if (not (`self.isWaveActive`))
        (`self.StartWave`)))))

(event `StartWave`
  (bind _spawnpoints (`self.spawnPoints`))
  (bind _returnvalue (`self.GetTransform` (`|GetArrayItem` _spawnpoints (`KismetMathLibrary.RandomIntegerInRange` 0 (`KismetArrayLibrary.Array_LastIndex` _spawnpoints)))))
  (`KismetSystemLibrary.PrintString` "WAVE STARTED")
  (set `self.isWaveActive` true)
  (set `self.enemiesAlive` 0)
  (`/Game/MyGame/UI/WB_WaveUI.ShowWaveStarted` (`/Game/MyGame/Blueprints/MyCharacter/BP_FirstPersonCharacter.waveUIRef` (`self.playerRef`)) (`self.waveNumber`))
  (for _ (range (+ (`KismetMathLibrary.FTrunc` (- (`self.enemiesToSpawn`) 1.0)) 1))
    (bind _returnvalue_2 (`|SpawnActorFromClass` "/Game/MyGame/Blueprints/EnemyAI/BP_EnemyAI.BP_EnemyAI_C" (`KismetMathLibrary.MakeTransform` (`KismetMathLibrary.MakeVector` (+ (.x (.location _returnvalue)) (`KismetMathLibrary.RandomFloatInRange` -200.0 200.0)) (.y (.location _returnvalue)) (+ (.z (.location _returnvalue)) 100.0)) (.rotation _returnvalue) (.scale _returnvalue)) "AdjustIfPossibleButAlwaysSpawn" "MultiplyWithRoot" null null))
    (add `/Game/MyGame/Blueprints/EnemyAI/BP_EnemyAI.OnEnemyDied` _returnvalue_2 (delegate `OnEnemyDied_Event`))
    (bind _result (`/Engine/EditorBlueprintResources/StandardMacros.IncrementInt` (`self.enemiesAlive`))
      (:`  `
        (bind _output_get (set `self.enemiesAlive` _result))
        (`/Game/MyGame/UI/WB_WaveUI.ShowEnemiesRemaining` (`/Game/MyGame/Blueprints/MyCharacter/BP_FirstPersonCharacter.waveUIRef` (`self.playerRef`)) _output_get)))))

(event `OnEnemyDied_Event`
  (bind _waveuiref (`/Game/MyGame/Blueprints/MyCharacter/BP_FirstPersonCharacter.waveUIRef` (`self.playerRef`)))
  (bind _result (`/Engine/EditorBlueprintResources/StandardMacros.DecrementInt` (`self.enemiesAlive`))
    (:`  `
      (bind _output_get (set `self.enemiesAlive` _result))
      (`/Game/MyGame/UI/WB_WaveUI.ShowEnemiesRemaining` (`/Game/MyGame/Blueprints/MyCharacter/BP_FirstPersonCharacter.waveUIRef` (`self.playerRef`)) (`self.enemiesAlive`))
      (if (== _output_get 0)
        (`self.EndWave`)
        (`KismetSystemLibrary.PrintString` "WAVE ENDED")
        (`/Game/MyGame/UI/WB_WaveUI.ShowWaveCompleted` _waveuiref)
        (`/Game/MyGame/UI/WB_WaveUI.HideEnemiesRemaining` _waveuiref)
        (`/Game/MyGame/UI/WB_WaveUI.UpdateWaveCompletedCount` _waveuiref (- (`self.waveNumber`) 1))))))

(event `EndWave`
  (`KismetSystemLibrary.PrintString` "WAVE ENDED")
  (set `self.isWaveActive` false)
  (bind _result (`/Engine/EditorBlueprintResources/StandardMacros.IncrementInt` (`self.waveNumber`))
    (:`  `
      (set `self.waveNumber` _result)
      (set `self.enemiesToSpawn` (+ (`self.enemiesToSpawn`) 2.0)))))

(fn `UserConstructionScript`)