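; BP_Gate is a double-door gate that swings shut after the first-person character leaves its trigger box.
; End overlap waits a short delay, then reverses two timelines that lerp each door's relative yaw from open to closed.
; A matching opening branch with its own timelines exists but is unconnected, and begin overlap is empty, so nothing here opens the gate.
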(event `self.Box.OnComponentBeginOverlap`
  (params (OverlappedComponent :type "PrimitiveComponent Object Reference") (OtherActor :type "Actor Object Reference") (OtherComp :type "PrimitiveComponent Object Reference") (OtherBodyIndex :type Integer) (bFromSweep :type Boolean) (SweepResult :type "HitResult Structure (by ref)")))

(event `self.Box.OnComponentEndOverlap`
  (params (OverlappedComponent :type "PrimitiveComponent Object Reference") (OtherActor :type "Actor Object Reference") (OtherComp :type "PrimitiveComponent Object Reference") (OtherBodyIndex :type Integer))
  (cast `/Game/MyGame/Blueprints/MyCharacter/BP_FirstPersonCharacter` OtherActor)
  (`KismetSystemLibrary.Delay` 3.0)
  ; Doors Close
  (`|ExecutionSequence`
    (:`then_0`
      (bind (_direction _left_door_open) (`Timeline|Timeline` :!via `ReverseFromEnd`)
        (:`Update`
          (`SceneComponent.K2_SetRelativeRotation` (`self.LeftDoor`) (`KismetMathLibrary.MakeRotator` 0.0 0.0 (`KismetMathLibrary.Lerp` (`self.leftDoorCloseValue`) (`self.leftDoorOpenValue`) _left_door_open)) false false))))
    (:`then_1`
      (bind (_direction_2 _right_door_open) (`Timeline|Timeline_0` :!via `ReverseFromEnd`)
        (:`Update`
          (`SceneComponent.K2_SetRelativeRotation` (`self.RightDoor`) (`KismetMathLibrary.MakeRotator` 0.0 0.0 (`KismetMathLibrary.Lerp` (`self.rightDoorCloseValue`) (`self.rightDoorOpenValue`) _right_door_open)) false false))))))

(fn `UserConstructionScript`)