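; BP_CoinSpawner is a spawner that scatters BP_Coin actors over the surfaces beneath a Box volume when play begins.
; A DoN node wired back on itself loops SpawnCoin up to AmountOfCoins times.
; SpawnCoin line-traces on Visibility from a random point within half the box extent toward a fixed low Z, with debug drawing.
; Each hit spawns a coin at the hit location; misses are not retried.
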(event `self.ReceiveBeginPlay`
  (bind _counter (`/Engine/EditorBlueprintResources/StandardMacros.Do N` (`self.amountOfCoins`) :!label _label)
    (:`Exit`
      (`self.SpawnCoin`)
      (if (not (== _counter (`self.amountOfCoins`)))
        (goto _label)))))

(fn `SpawnCoin`
  (bind _returnvalue (`KismetMathLibrary.RandomPointInBoundingBox` (`SceneComponent.K2_GetComponentLocation` (`self.Box`)) (`KismetMathLibrary.MakeVector` (/ (.x (`BoxComponent.GetUnscaledBoxExtent` (`self.Box`))) 2.0) (/ (.y (`BoxComponent.GetUnscaledBoxExtent` (`self.Box`))) 2.0) (/ (.z (`BoxComponent.GetUnscaledBoxExtent` (`self.Box`))) 2.0))))
  (bind (_outhit _returnvalue_2) (`KismetSystemLibrary.LineTraceSingle` :`Start` _returnvalue :`End` (`KismetMathLibrary.MakeVector` (.x _returnvalue) (.y _returnvalue) -2000.0) :`TraceChannel` "TraceTypeQuery1" :`DrawDebugType` "ForDuration"))
  (if _returnvalue_2
    (`|SpawnActorFromClass` "/Game/MyGame/Blueprints/BP_Coin.BP_Coin_C" (`KismetMathLibrary.MakeTransform` (`.Location` (`GameplayStatics.BreakHitResult` _outhit))) "Undefined" "MultiplyWithRoot" null null)))

(fn `UserConstructionScript`)